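; BP_Enemy is an enemy character that can be marked as focused and killed with a physical impulse.
; Focus events show or hide a FocusArrow component above or on the enemy.
; Death turns the mesh into a ragdoll by simulating physics, applies the given impulse, and sets the capsule to NoCollision.
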(event `FocusEnemy`
  (`SceneComponent.SetHiddenInGame` (`self.FocusArrow`) false false))

(event `ClearFocus`
  (`SceneComponent.SetHiddenInGame` (`self.FocusArrow`) true false))

(event `Die`
  (params (Impulse :type "Vector Structure"))
  (`PrimitiveComponent.SetSimulatePhysics` (`self.Mesh`) true)
  (`PrimitiveComponent.AddImpulse` (`self.Mesh`) Impulse "None" false)
  (`PrimitiveComponent.SetCollisionProfileName` (`self.CapsuleComponent`) "NoCollision" true))

(fn `UserConstructionScript`)