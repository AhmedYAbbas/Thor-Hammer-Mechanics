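; Mjolnir hammer actor that the player throws to fly through a chain of enemies and return.
; A timeline lerps each leg at a play rate scaled by distance for constant speed, restarting for each queued enemy.
; The final leg tracks the player's live location, then notifies BP_Player on arrival.
; Collision, spin and air audio run during flight, and overlapped enemies die with a directional impulse and lightning effect.
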(event `self.ReceiveBeginPlay`
  ;[1 1 1] Get Player Reference
  (bind _asbp_player (cast `/Game/ITIGame/Player/BP_Player` (`GameplayStatics.GetPlayerCharacter` 0)))
  (set `self.PlayerRef` _asbp_player)
  (`self.SetActorEnableCollision` false))

(event `StartFollow`
  (bind _returnvalue (`self.CalculatePlayRate`))
  (bind _output (`|GetArrayItem` (`self.Enemies`)))
  (set `self.StartPos` (`self.K2_GetActorLocation`))
  (if (> _returnvalue 0.0)
    (`TimelineComponent.SetPlayRate` (`self.ThrowTimeline`) _returnvalue)
    (bind (_direction _alpha) (`Timeline|ThrowTimeline` :!via `PlayFromStart`)
      (:`Update`
        ;[1 1 1] Update (Lerp) Mjolnir Location
        (`self.K2_SetActorLocation` (`KismetMathLibrary.VLerp` (`self.StartPos`) (`self.GetCorrectEndPoint`) _alpha)))
      (:`Finished`
        (if (not (`KismetArrayLibrary.Array_IsEmpty` (`self.Enemies`))) :!label _label
          (set `self.EndPos` (`self.K2_GetActorLocation` _output))
          (`KismetArrayLibrary.Array_RemoveItem` (`self.Enemies`) _output)
          (`self.StartFollow`)
          (elif (not (`self.IsFinalLoop`))
            ;[1 1 1] Start Final Loop Return To Player
            (set `self.IsFinalLoop` true)
            (`self.StartFollow`)
            (`/Game/ITIGame/Player/BP_Player.MjolnirTowardPlayer` (`self.PlayerRef`))
            (else
              ;[1 1 1] Shield Reached Player
              (set `self.IsFinalLoop` false)
              (`GameplayStatics.PlaySoundAtLocation` "/Game/ITIGame/Audio/MS_GrabMjolnir.MS_GrabMjolnir" (`self.K2_GetActorLocation`) (struct) 1.0 1.0 0.0 null null null null)
              (`AudioComponent.SetVolumeMultiplier` (`self.LoopingAirAudio`) 0.0)
              (set `RotatingMovementComponent.RotationRate` (struct) (`self.RotatingMovement`))
              (`self.SetActorEnableCollision` false)
              (`/Game/ITIGame/Player/BP_Player.MjolnirCompleted` (`self.PlayerRef`)))))))
    (else
      (goto _label))))

(event `ThrowMjolnir`
  (params (EnemiesArray :type "Array of /Game/ITIGame/Enemy/BP_Enemy Object Reference") (EndPointParam :type "Vector Structure"))
  ;[1 1 1] Throw Mjolnir
  (if (`KismetArrayLibrary.Array_IsEmpty` (`self.Enemies`))
    (set `self.Enemies` EnemiesArray)
    (set `self.EndPos` EndPointParam)
    (else
      (set `self.StartPos` (`self.K2_GetActorLocation` (`|GetArrayItem` (`self.Enemies`))))))
  (`self.K2_DetachFromActor` "KeepWorld" "KeepWorld" "KeepWorld")
  (`AudioComponent.SetVolumeMultiplier` (`self.LoopingAirAudio`) 0.2)
  (set `RotatingMovementComponent.RotationRate` (struct :`Pitch` 1500.0) (`self.RotatingMovement`))
  (`self.SetActorEnableCollision` true)
  (`self.StartFollow`))

(event `self.StaticMesh.OnComponentBeginOverlap`
  (params (OverlappedComponent :type "PrimitiveComponent Object Reference") (OtherActor :type "Actor Object Reference") (OtherComp :type "PrimitiveComponent Object Reference") (OtherBodyIndex :type Integer) (bFromSweep :type Boolean) (SweepResult :type "HitResult Structure (by ref)"))
  (bind _asbp_enemy (cast `/Game/ITIGame/Enemy/BP_Enemy` OtherActor))
  (`/Game/ITIGame/Enemy/BP_Enemy.Die` _asbp_enemy (* (`KismetMathLibrary.Normal` (- (`self.EndPos`) (`self.StartPos`))) 1000000.0))
  (`NiagaraFunctionLibrary.SpawnSystemAtLocation` "/Game/ITIGame/Hack_And_Slash_FX/VFX_Niagara/Impacts/NS_Lightning_Slash_Impact.NS_Lightning_Slash_Impact" (`self.K2_GetActorLocation`)))

(fn `CalculatePlayRate`
  (returns (ReturnValue :type "Float (double-precision)"))
  (return (/ (`self.FlightSpeed`) (`KismetMathLibrary.Vector_Distance` (`self.StartPos`) (`self.GetCorrectEndPoint`)))))

(fn `GetCorrectEndPoint`
  (returns (ReturnValue :type "Vector Structure"))
  (return (select `bool` (`self.IsFinalLoop`) :`false` (`self.EndPos`) :`true` (`self.K2_GetActorLocation` (`self.PlayerRef`)))))

(fn `UserConstructionScript`)